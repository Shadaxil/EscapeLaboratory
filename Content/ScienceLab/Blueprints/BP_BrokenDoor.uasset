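; BP_BrokenDoor is a two-panel lab sliding door whose movement logic is broken as wired.
; Collision overlap begin and end toggle AutoOpen and AutoClose, which Tick uses to step DoorPosition.
; Opening raises the value to 90 without moving either panel.
; Closing offsets the panels oppositely only above 90, resets the value without moving them at exactly 90, and does nothing below.
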(event `self.ReceiveTick`
  (params (DeltaSeconds :type "Float (single-precision)"))
  (bind _door_position (`self.Door Position`))
  (bind _door_position_2 (`self.Door Position`))
  (bind _door_position_3 (`self.Door Position`))
  ;[0 0.3281 0] SecurityBreach0X00CF52
  (if (`self.Auto Open`)
    (`/Engine/EditorBlueprintResources/StandardMacros.CompareFloat` _door_position_2 90.0
      (:`==`
        (set `self.Door Position` 90.0))
      (:`<`
        (set `self.Door Position` (+ _door_position_2 4.0))))
    (elif (`self.Auto Close`)
      (`/Engine/EditorBlueprintResources/StandardMacros.CompareFloat` _door_position 90.0
        (:`>`
          (set `self.Door Position` (- _door_position 4.0))
          (`SceneComponent.K2_SetRelativeLocation` (`self.LabDoor03B`) (`KismetMathLibrary.MakeVector` 0.0 _door_position_3) false false)
          (`SceneComponent.K2_SetRelativeLocation` (`self.LabDoor03A`) (`KismetMathLibrary.MakeVector` 0.0 (* _door_position_3 -1.0)) false false))
        (:`==`
          (set `self.Door Position` 0.0)
          (set `self.Auto Close` false))))))

(event `self.Collision.OnComponentBeginOverlap`
  (params (OverlappedComponent :type "PrimitiveComponent Object Reference") (OtherActor :type "Actor Object Reference") (OtherComp :type "PrimitiveComponent Object Reference") (OtherBodyIndex :type Integer) (bFromSweep :type Boolean) (SweepResult :type "HitResult Structure (by ref)"))
  ;[0 0.3281 0] SecurityBreach0X00CF52
  (set `self.Auto Open` true)
  (set `self.Auto Close` false))

(event `self.Collision.OnComponentEndOverlap`
  (params (OverlappedComponent :type "PrimitiveComponent Object Reference") (OtherActor :type "Actor Object Reference") (OtherComp :type "PrimitiveComponent Object Reference") (OtherBodyIndex :type Integer))
  ;[0 0.3281 0] SecurityBreach0X00CF52
  (set `self.Auto Open` false)
  (set `self.Auto Close` true))

(fn `UserConstructionScript`)